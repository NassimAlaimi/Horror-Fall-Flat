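; BP_Item is a pickup actor for the inventory system, with its mesh set from ItemModel in the construction script.
; PickUpItem returns the Item data and triggers DestroyItem, which removes the Trigger, shrinks the model with a timeline, plays a pickup sound once and destroys the actor after a short delay.
; Tick clears the model's custom depth whenever it is on, so any such highlight must be reapplied externally.
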(event Custom|Destroy%20Item
  (Components|DestroyComponent (Variables|Default|GetTrigger))
  (Utilities|FlowControl|DelayUntilNextTick)
  (bind _shrinktimeline (Timeline|Shrink PlayFromStart)
    (:Update
      (Transformation|SetWorldScale3D (Variables|Default|GetModel) (Math|Conversions|ToVector(Float) (Math|Float|Lerp 1.0 0.0 _shrinktimeline)))
      (Utilities|FlowControl|DoOnce false
        (:Completed
          (Audio|PlaySound2D "/Engine/VREditor/Sounds/UI/Object_PickUp.Object_PickUp" 1.0 1.0 0.0 0 0)
          (Utilities|FlowControl|Delay 0.4)
          (Actor|DestroyActor))))))

(event EventTick
  (params (DeltaSeconds :type Float%20%28single-precision%29))
  (if (Variables|/Script/Engine.PrimitiveComponent|GetbRenderCustomDepth (Variables|Default|GetModel))
    (Rendering|SetRenderCustomDepth (Variables|Default|GetModel) false)))

(fn ConstructionScript
  (Components|StaticMesh|SetStaticMesh (Variables|Default|GetModel) (Variables|Default|GetItemModel)))

(fn PickUpItem
  (CallFunction|DestroyItem)
  (return (Variables|Default|GetItem)))