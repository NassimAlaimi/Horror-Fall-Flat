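; BP_Drawer is an interactable hiding spot that the player enters and leaves through a hinged door.
; Interact toggles Inside, sets IsHidden on BP_Player, moves the player to the REFInside transform in both directions, and snaps the door closed or open.
; The Trigger overlap shows and removes an interact prompt widget for the player.
; Tick clears the door's custom-depth highlight whenever it is set.
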(event OnComponentBeginOverlap(trigger)
  (params (OverlappedComponent :type Primitive%20Component%20Object%20Reference) (OtherActor :type Actor%20Object%20Reference) (OtherComp :type Primitive%20Component%20Object%20Reference) (OtherBodyIndex :type Integer) (bFromSweep :type Boolean) (SweepResult :type Hit%20Result%20Structure%20%28by%20ref%29))
  ;[1 0.4354 0.9294] Screen Prompt "Press ... to Interact"
  (if (== OtherActor (Game|GetPlayerCharacter 0))
    (UserInterface|Viewport|AddtoViewport (Variables|Default|GetInteractPromp) 0)))

(event OnComponentEndOverlap(trigger)
  (params (OverlappedComponent :type Primitive%20Component%20Object%20Reference) (OtherActor :type Actor%20Object%20Reference) (OtherComp :type Primitive%20Component%20Object%20Reference) (OtherBodyIndex :type Integer))
  ;[1 0.4354 0.9294] Screen Prompt "Press ... to Interact"
  (if (== (Game|GetPlayerCharacter 0) OtherActor)
    (Widget|RemovefromParent (Variables|Default|GetInteractPromp))))

(event EventBeginPlay
  ;[1 0.4354 0.9294] Screen Prompt "Press ... to Interact"
  (bind _returnvalue (UserInterface|CreateWidget "/Game/Blueprints/Drawer/WBP_interact.WBP_interact_C"))
  (Variables|Default|SetInteractPromp _returnvalue))

(event Collision|EventActorBeginOverlap
  (params (OtherActor :type Actor%20Object%20Reference)))

(event EventTick
  (params (DeltaSeconds :type Float%20%28single-precision%29))
  ;[0.957 0.4827 1] Remove hightlight
  (if (Variables|/Script/Engine.PrimitiveComponent|GetbRenderCustomDepth (Variables|Default|GetDoor))
    (Rendering|SetRenderCustomDepth (Variables|Default|GetDoor) false)))

(event EventInteract
  ;[1 0.4308 0.9567] Open & Close the Door
  (if (not (Variables|Default|Getinside))
    (CallFunction|Open/ClosetheDoor true "0, 0, 0")
    (else
      (CallFunction|Open/ClosetheDoor false "0.000000,120.000000,0.000000"))))

(fn ConstructionScript)

(fn Open/ClosetheDoor
  (params (isInside :type Boolean) (rotation :type Rotator))
  (bind _ref_inside (Variables|Default|GetREF_Inside))
  (bind _returnvalue (Transformation|GetWorldTransform _ref_inside))
  (Variables|Default|Setinside isInside)
  (bind _asbp_player (Utilities|Casting|CastToBP_Player (Game|GetPlayerCharacter 0)))
  (Variables|/Game/Blueprints/Player/BP_Player.BP_Player_C|SetisHidden _asbp_player isInside)
  (Transformation|SetActorTransform (Game|GetPlayerCharacter 0) (Math|Transform|MakeTransform (.location _returnvalue) (.rotation _returnvalue) (.scale _returnvalue)))
  (Transformation|SetRelativeRotation (Variables|Default|GetDoor) rotation false false))