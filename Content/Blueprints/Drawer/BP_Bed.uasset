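; BP_Bed is an interactable bed that moves the player in and out of it.
; Each Interact event flips the IsInside flag and snaps player character 0 to the full transform of the RefInside or RefOutside reference.
; It also toggles the character mesh, making it visible on entry and hidden on exit, with no animation or blending.
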(event EventBeginPlay)

(event Collision|EventActorBeginOverlap
  (params (OtherActor :type Actor%20Object%20Reference)))

(event EventTick
  (params (DeltaSeconds :type Float%20%28single-precision%29)))

(event EventInteract
  (bind _ref_inside (Variables|Default|GetRef_Inside))
  (bind _ref_outside (Variables|Default|GetRef_Outside))
  (bind _returnvalue (Transformation|GetWorldTransform _ref_outside))
  (bind _returnvalue_2 (Transformation|GetWorldTransform _ref_inside))
  (if (not (Variables|Default|GetisInside))
    (Variables|Default|SetisInside true)
    (Transformation|SetActorTransform (Game|GetPlayerCharacter 0) (Math|Transform|MakeTransform (.location _returnvalue_2) (.rotation _returnvalue_2) (.scale _returnvalue_2)))
    (Rendering|SetVisibility (Variables|/Script/Engine.Character|GetMesh (Game|GetPlayerCharacter 0)) true false)
    (else
      (Variables|Default|SetisInside false)
      (Transformation|SetActorTransform (Game|GetPlayerCharacter 0) (Math|Transform|MakeTransform (.location _returnvalue) (.rotation _returnvalue) (.scale _returnvalue)))
      (Rendering|SetVisibility (Variables|/Script/Engine.Character|GetMesh (Game|GetPlayerCharacter 0)) false false))))

(fn ConstructionScript)