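; BP_FallingPlatform is a platform that falls shortly after the player character steps on it, then comes back.
; A box overlap triggers timed orange and red material warnings with sounds, then enables physics on the mesh.
; After a delay, ShouldRespawn chooses between spawning a replacement at the saved transform and destroying itself, or a deprecated in-place reset of physics, position and material.
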(event OnComponentBeginOverlap(Box)
  (params (OverlappedComponent :type Primitive%20Component%20Object%20Reference) (OtherActor :type Actor%20Object%20Reference) (OtherComp :type Primitive%20Component%20Object%20Reference) (OtherBodyIndex :type Integer) (bFromSweep :type Boolean) (SweepResult :type Hit%20Result%20Structure%20%28by%20ref%29))
  ;[0.4678 0.1285 0] Features - Falling Platform
  ;;[1 1 1] On character step on cube
  (if (and (== OtherActor (Game|GetPlayerCharacter 0)) (Variables|Default|GetIsActive?))
    (Variables|Default|SetIsActive? false)
    ;;;[1 1 1] 1. Anticipation - Change color to orange
    (CallFunction|ChangeColorandPlaySound "/Game/Materials/MI_Orange_Inst.MI_Orange_Inst" "/Engine/VREditor/Sounds/UI/Flashlight_Switch.Flashlight_Switch")
    (Utilities|FlowControl|Delay 1.1)
    ;;;[1 1 1] 2. Just before falling - Change color to red
    (CallFunction|ChangeColorandPlaySound "/Game/Materials/MI_Red_Inst.MI_Red_Inst" "/Engine/VREditor/Sounds/UI/Click_on_Button.Click_on_Button")
    (Utilities|FlowControl|Delay 0.9)
    (CallFunction|MakePlatformFalls)))

(event Custom|ChangeColorAndPlaySound
  (params (MaterialToSet :type Material%20Interface%20Object%20Reference) (SFXToPlay :type Sound%20Base%20Object%20Reference))
  ;[0.4678 0.1285 0] Features - Falling Platform
  ;;[1 1 1] Set material - play vfx
  (Rendering|Material|SetMaterial (Variables|Default|GetStaticMesh) 0 MaterialToSet)
  (Audio|PlaySound2D SFXToPlay 1.0 1.0 0.0 0 0))

(event Custom|MakePlatformFalls
  ;[0.4678 0.1285 0] Features - Falling Platform
  ;;[1 1 1] Play vfx - enable phyics
  (Audio|PlaySound2D "/Engine/VREditor/Sounds/UI/Dockable_Window_Close.Dockable_Window_Close" 1.0 1.0 0.0 0 0)
  (Physics|SetSimulatePhysics (Variables|Default|GetStaticMesh) true)
  (Utilities|FlowControl|Delay 5.0)
  (if (Variables|Default|GetShouldRespawn?)
    (CallFunction|RespawnPlatform)
    (else
      (CallFunction|RespawnPlatformatDefaultLoc))))

(event Custom|RespawnPlatformAtDefaultLoc
  (bind _staticmesh (Variables|Default|GetStaticMesh))
  ;[0.4678 0.1285 0] Features - Falling Platform
  ;;[1 1 1] DEPRECATED - disable physics - tp the static mesh to default location - set material to default
  (Physics|SetSimulatePhysics _staticmesh false)
  (Transformation|SetWorldLocationAndRotation _staticmesh (Variables|Default|GetDefaultLocation) (Variables|Default|GetDefaultRotation) false false)
  (Variables|Default|SetIsActive? true)
  (Rendering|Material|SetMaterial (Variables|Default|GetStaticMesh) 0 "/Game/Materials/MI_Blue_Inst.MI_Blue_Inst"))

(event Custom|RespawnPlatform
  ;[0.4678 0.1285 0] Features - Falling Platform
  ;;[1 1 1] Spawn new falling platform at default loc / rot then destroy the current falling platform
  (Game|SpawnActorfromClass "BP_FallingPlatform_C" (Math|Transform|MakeTransform (Variables|Default|GetDefaultLocation) (Variables|Default|GetDefaultRotation) (Transformation|GetActorScale3D)) "Undefined" "MultiplyWithRoot" 0 0)
  (Actor|DestroyActor))

(event EventBeginPlay
  (bind _staticmesh (Variables|Default|GetStaticMesh))
  ;[0.04971 0.2086 1] Save default location of the static mesh (cube)
  (Variables|Default|SetDefaultLocation (Transformation|GetWorldLocation _staticmesh))
  (Variables|Default|SetDefaultRotation (Transformation|GetWorldRotation _staticmesh)))

(fn ConstructionScript)