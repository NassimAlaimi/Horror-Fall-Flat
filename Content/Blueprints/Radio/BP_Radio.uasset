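; Interactable radio that toggles on and off with switch sounds and emits noise that AI pawn sensing can hear.
; Turning on randomly starts Station1 or, far more often, the Emergency broadcast; turning off stops both.
; While on, a looping timer repeats the noise at the radio's location, attributed to the player pawn.
; A second looping timer clears the custom-depth outline.
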(event Custom|turnRadio%20Off
  ;[1 1 1] Turn off the Radio
  (Audio|PlaySoundatLocation "/Game/Blueprints/Radio/Audio/Vintage_RadioTurn_Off_Sound_Effect.Vintage_RadioTurn_Off_Sound_Effect" (Transformation|GetWorldLocation (Variables|Default|GetRadio)) "0, 0, 0" 1.0 1.0 0.0 0 0 0 0)
  (Audio|Components|Audio|Stop (Variables|Default|GetStation_1))
  (Variables|Default|SetIs_Radio_On false)
  (if (Variables|/Script/Engine.PrimitiveComponent|GetbRenderCustomDepth (Variables|Default|GetRadio))
    (Rendering|SetRenderCustomDepth (Variables|Default|GetRadio) false)))

(event Custom|Remove%20Outlline
  (if (Variables|/Script/Engine.PrimitiveComponent|GetbRenderCustomDepth (Variables|Default|GetRadio))
    (Rendering|SetRenderCustomDepth (Variables|Default|GetRadio) false)))

(event Custom|Make%20Noise
  (if (Variables|Default|GetIs_Radio_On)
    (Class|PawnNoiseEmitterComponent|MakeNoise (Variables|Default|GetPawnNoiseEmitter) (Game|Player|GetPlayerPawn 0) 1.0 (Transformation|GetWorldLocation (Variables|Default|GetRadio)))))

(event Custom|Toggle%20Radio%20ON%20OFF
  ;[1 1 1] Swich On/Off
  (if (Variables|Default|GetIs_Radio_On)
    (CallFunction|TurnRadioOff)
    (else
      (CallFunction|TurnRadioon))))

(event Custom|Turn%20Radio%20On
  ;[1 1 1] Turn On the Radio
  (Audio|PlaySoundatLocation "/Game/Blueprints/Radio/Audio/Vintage_RadioTurn_On_Sound_Effect.Vintage_RadioTurn_On_Sound_Effect" (Transformation|GetWorldLocation (Variables|Default|GetRadio)) "0, 0, 0" 1.0 1.0 0.0 0 0 0 0)
  (Utilities|FlowControl|Delay 0.5)
  (switch int (Math|Random|RandomIntegerinRange 0 4)
    (:0
      (Audio|Components|Audio|Play (Variables|Default|GetStation_1) 0.0))
    (:1
      (Audio|Components|Audio|Play (Variables|Default|GetEmergency) 0.0 :!label _label))
    (:2
      (goto _label))
    (:3
      (goto _label))
    (:4
      (goto _label)))
  (Variables|Default|SetIs_Radio_On true)
  (Class|PawnNoiseEmitterComponent|MakeNoise (Variables|Default|GetPawnNoiseEmitter) (Game|Player|GetPlayerPawn 0) 1.0 (Transformation|GetWorldLocation (Variables|Default|GetRadio))))

(event EventBeginPlay
  (Utilities|Time|SetTimerbyEvent (delegate Custom|Make%20Noise) 15.0 true)
  (Utilities|Time|SetTimerbyEvent (delegate Custom|Remove%20Outlline) 1.0 true))

(event EventInteract
  ;[1 1 1] Interact with the radio
  (CallFunction|ToggleRadioONOFF))

(fn ConstructionScript)