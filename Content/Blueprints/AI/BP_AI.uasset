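; BP_AI is an AI pawn that turns sight and hearing into Blackboard state for chasing the player and investigating sounds.
; PawnSensing sets a seen-player flag when it spots BP_Player, and a looping timer periodically clears it so the flag lapses unless sight refreshes it.
; Heard noises write their X and Y location as separate floats and raise the heard-sound and radio-on flags, which this Blueprint never clears.
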(event OnSeePawn(PawnSensing)
  (params (Pawn :type Pawn%20Object%20Reference))
  ;[0.364 1 0.2355] Trigger chase player on see pawn
  (Utilities|Casting|CastToBP_Player Pawn)
  (AI|Components|Blackboard|SetValueasBool (AI|GetBlackboard (AI|GetAIController self)) (Utilities|Name|MakeLiteralName "asSeenPlayer") (Utilities|IsValid Pawn)))

(event OnHearNoise(PawnSensing)
  (params (Instigator :type Pawn%20Object%20Reference) (Location :type Vector%20%28by%20ref%29 :default "0, 0, 0") (Volume :type Float%20%28single-precision%29))
  (bind _self self)
  (bind _returnvalue (AI|GetAIController _self))
  (bind _returnvalue_2 (AI|GetBlackboard _returnvalue))
  ;[0.4095 1 0.3075] Trigger Investigate Sound
  (AI|Components|Blackboard|SetValueasFloat _returnvalue_2 (Utilities|Name|MakeLiteralName "xLocation") (.x Location))
  (AI|Components|Blackboard|SetValueasFloat _returnvalue_2 (Utilities|Name|MakeLiteralName "yLocation") (.y Location))
  (AI|Components|Blackboard|SetValueasBool _returnvalue_2 (Utilities|Name|MakeLiteralName "asHearedSound") true)
  (AI|Components|Blackboard|SetValueasBool (AI|GetBlackboard (AI|GetAIController self)) (Utilities|Name|MakeLiteralName "isRadioOn") true))

(event Custom|Stop%20Seeing%20Player
  ;[0.3676 1 0.3103] Check if player is still in the detection Range
  (AI|Components|Blackboard|SetValueasBool (AI|GetBlackboard (AI|GetAIController self)) (Utilities|Name|MakeLiteralName "asSeenPlayer") false))

(event EventBeginPlay
  ;[0.3676 1 0.3103] Check if player is still in the detection Range
  (Variables|Default|SetisScreaming false)
  (Variables|Default|SetisCrouching false)
  (Utilities|Time|SetTimerbyEvent (delegate Custom|Stop%20Seeing%20Player) 4.0 true))

(fn ConstructionScript)